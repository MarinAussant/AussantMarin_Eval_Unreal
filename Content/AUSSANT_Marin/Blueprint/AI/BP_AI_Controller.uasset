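; AI controller that sends its AI after the player through a behavior tree and blackboard.
; BeginPlay initializes BB_AI_Blackboard and keeps its component.
; AiMoveToPlayer runs BT_AI_BehaviorTree and writes player 0's current location to the PlayerPosition key, a snapshot taken only when the function is called.
; PlayerDistance only assigns its input to a same-named value, and nothing in this graph calls either function.
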(event EventBeginPlay
  (bind _blackboardcomponent (Class|AIController|UseBlackboard "/Game/AUSSANT_Marin/Blueprint/AI/BB_AI_Blackboard.BB_AI_Blackboard"))
  (Variables|Default|SetBlackboard%20Component _blackboardcomponent))

(fn ConstructionScript)

(fn PlayerDistance
  (params (playerDistance :type Float%20%28double-precision%29))
  (Variables|Default|SetPlayer%20Distance playerDistance))

(fn AiMovetoPlayer
  (AI|RunBehaviorTree "/Game/AUSSANT_Marin/Blueprint/AI/BT_AI_BehaviorTree.BT_AI_BehaviorTree")
  (AI|Components|Blackboard|SetValueasVector (Variables|Default|GetBlackboard%20Component) (Utilities|Name|MakeLiteralName "PlayerPosition") (Transformation|GetActorLocation (Game|GetPlayerCharacter 0))))