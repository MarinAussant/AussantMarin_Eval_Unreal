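; BP_AICharacter is an enemy AI character that chases the player at close range and restarts the level when it touches them.
; Each Tick it measures the 2D distance from its capsule to the player and, within a fixed radius, calls AiMoveToPlayer on its BP_AI_Controller.
; A capsule hit against BP_ThirdPersonCharacter reopens the current level by name.
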(event OnComponentHit(CapsuleComponent)
  (params (HitComponent :type Primitive%20Component%20Object%20Reference) (OtherActor :type Actor%20Object%20Reference) (OtherComp :type Primitive%20Component%20Object%20Reference) (NormalImpulse :type Vector :default "0, 0, 0") (Hit :type Hit%20Result%20Structure%20%28by%20ref%29))
  (Utilities|Casting|CastToBP_ThirdPersonCharacter OtherActor)
  (bind _returnvalue (Game|GetCurrentLevelName true))
  (Game|OpenLevel(byName) (Utilities|String|StringToName _returnvalue)))

(event EventTick
  (params (DeltaSeconds :type Float%20%28single-precision%29))
  ;[1 1 1] Calcul la distance avec le joueur
  (bind _asbp_ai_controller (Utilities|Casting|CastToBP_AI_Controller (Pawn|GetController self)))
  (if (<= (Math|Vector|Distance2D(Vector) (Transformation|GetWorldLocation (Variables|Collision|GetCapsuleComponent)) (Transformation|GetActorLocation (Game|GetPlayerCharacter 0))) 4e+02)
    (Default|AiMovetoPlayer _asbp_ai_controller)))

(fn ConstructionScript)